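; Boost item actor that temporarily propels its owning ArcadeCar forward with smoke active.
; On BeginPlay it disables the car's CanMove, cuts its turning force and starts a looping substep timer calling AddBoost.
; AddBoost applies amplified forward force and damping only while grounded, so airborne time does not count toward the boost duration.
; Tick restores movement and turning, stops the smoke and destroys the item once BoostTime reaches LifeTime.
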(event `self.ReceiveBeginPlay`
  (`parent.ReceiveBeginPlay`)
  (bind _asarcade_car (cast `/Game/Blueprints/Car/ArcadeCar` (`self.GetOwner`)))
  (set `/Game/Blueprints/Car/ArcadeCar.CanMove` false _asarcade_car)
  (set `/Game/Blueprints/Car/ArcadeCar.turningForce` (/ (`/Game/Blueprints/Car/ArcadeCar.turningForce` _asarcade_car) 3.0) _asarcade_car)
  (`KismetSystemLibrary.K2_SetTimer` null "AddBoost" (`self.boostSubstep`) true)
  (`ActorComponent.SetActive` (`/Game/Blueprints/Car/ArcadeCar.Smoke` _asarcade_car) true false))

(event `self.ReceiveTick`
  (params (DeltaSeconds :type "Float (single-precision)"))
  (`parent.ReceiveTick` DeltaSeconds)
  (if (>= (`self.boostTime`) (`self.lifeTime`))
    (set `/Game/Blueprints/Car/ArcadeCar.CanMove` true (stale `self.ReceiveBeginPlay` _asarcade_car))
    (set `/Game/Blueprints/Car/ArcadeCar.turningForce` (* (`/Game/Blueprints/Car/ArcadeCar.turningForce` (stale `self.ReceiveBeginPlay` _asarcade_car)) 3.0) (stale `self.ReceiveBeginPlay` _asarcade_car))
    (`self.K2_DestroyActor`)
    (`ActorComponent.SetActive` (`/Game/Blueprints/Car/ArcadeCar.Smoke` (stale `self.ReceiveBeginPlay` _asarcade_car)) false false)))

(fn `AddBoost`
  (bind _asarcade_car (cast `/Game/Blueprints/Car/ArcadeCar` (`self.GetOwner`)))
  (if (`/Game/Blueprints/Car/ArcadeCar.IsTouchingGround` _asarcade_car)
    (bind _body (`/Game/Blueprints/Car/ArcadeCar.Body` _asarcade_car))
    (`PrimitiveComponent.SetLinearDamping` _body 3.0)
    (`PrimitiveComponent.AddForce` _body (* (* (`SceneComponent.GetForwardVector` _body) (`/Game/Blueprints/Car/ArcadeCar.forwardForce` _asarcade_car)) 1.5) "None" false)
    (set `self.boostTime` (+ (`self.boostTime`) (`self.boostSubstep`)))
    (else
      (`PrimitiveComponent.SetLinearDamping` _body 0.0))))

(fn `UserConstructionScript`
  (`parent.UserConstructionScript`))