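; Timed pickup that gives an overlapping ArcadeCar a random item, unless that car is in first place.
; The item comes from the first three entries of MasterGameObject's ItemArray and fills the first empty of two slots, destroying the pickup.
; A timeline scales it up on spawn, then a timer based on TimeToLive starts a dynamic-material dissolve that ends in destruction.
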(event `self.ReceiveBeginPlay`
  (bind _cube (`self.Cube`))
  (bind (_direction _scaling_factor) (`Timeline|Scale Up`)
    (:`Update`
      (`SceneComponent.SetWorldScale3D` (`self.DefaultSceneRoot`) (`KismetMathLibrary.MakeVector` _scaling_factor _scaling_factor _scaling_factor)))
    (:`Finished`
      ;[1 1 1] Object Fade Out Over Time
      (bind _returnvalue (`PrimitiveComponent.CreateDynamicMaterialInstance` _cube 0 (`PrimitiveComponent.GetMaterial` _cube 0)))
      (`KismetSystemLibrary.K2_SetTimerDelegate` (delegate `Set Fade Out`) (- (`self.TimeToLive`) 10.0)))))

(event `Set Fade Out`
  ;[1 1 1] Object Fade Out Over Time
  (bind (_direction _dissolve) (`Timeline|DissolveTimeline`)
    (:`Update`
      (`MaterialInstanceDynamic.SetScalarParameterValue` (stale `self.ReceiveBeginPlay` _returnvalue) "Dissolve Amount" _dissolve))
    (:`Finished`
      (`self.K2_DestroyActor`))))

(event `self.ReceiveActorBeginOverlap`
  (params (OtherActor :type "Actor Object Reference"))
  (bind _asarcade_car (cast `/Game/Blueprints/Car/ArcadeCar` OtherActor))
  (bind _outactors (`GameplayStatics.GetAllActorsOfClass` "/Game/Blueprints/MasterGameObject.MasterGameObject_C"))
  (bind _output (`|GetArrayItem` _outactors))
  ;[1 1 1] Is Player First Place?
  (if (not (== _asarcade_car (`/Game/Blueprints/MasterGameObject.firstPlacePlayer` _output)))
    ;[1 1 1] Is Item1 = None
    (if (== (`/Game/Blueprints/Car/ArcadeCar.Item1` _asarcade_car) "/Game/Blueprints/Item/Item_None.Item_None_C")
      (bind _output_2 (`|GetArrayItem` (`/Game/Blueprints/MasterGameObject.itemArray` _output) (`KismetMathLibrary.RandomInteger` 3)))
      (set `/Game/Blueprints/Car/ArcadeCar.Item1` _output_2 _asarcade_car)
      (`self.K2_DestroyActor` :!label _label)
      (else
        ;[1 1 1] Is Item2 = None
        (if (== (`/Game/Blueprints/Car/ArcadeCar.Item2` _asarcade_car) "/Game/Blueprints/Item/Item_None.Item_None_C")
          (set `/Game/Blueprints/Car/ArcadeCar.Item2` _output_2 _asarcade_car)
          (goto _label))))))

(fn `UserConstructionScript`)