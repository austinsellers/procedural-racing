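; Item actor for an arcade car game that temporarily reverses the controls of every player except its owner.
; On BeginPlay it reads the player list from MasterGameObject and sets ReverseControls on each other player's ArcadeCarController.
; A one-shot timer clears the flag after eight seconds and destroys the item.
; An AddBoost function that pushes the grounded owner car forward is defined but not called in this graph.
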(event `self.ReceiveBeginPlay`
  (`parent.ReceiveBeginPlay`)
  (bind _outactors (`GameplayStatics.GetAllActorsOfClass` "/Game/Blueprints/MasterGameObject.MasterGameObject_C"))
  (for _array_element (`/Game/Blueprints/MasterGameObject.playerList` (`|GetArrayItem` _outactors))
    (if (!= _array_element (`self.GetOwner`))
      (bind _asarcade_car_controller (cast `/Game/Blueprints/Car/ArcadeCarController` (`Pawn.GetController` _array_element)))
      (set `/Game/Blueprints/Car/ArcadeCarController.ReverseControls` true _asarcade_car_controller)))
  (`KismetSystemLibrary.K2_SetTimerDelegate` (delegate `ReverseControls`) 8.0))

(event `ReverseControls`
  (for _array_element (`/Game/Blueprints/MasterGameObject.playerList` (`|GetArrayItem` (stale `self.ReceiveBeginPlay` _outactors)))
    (if (!= _array_element (`self.GetOwner`))
      (bind _asarcade_car_controller (cast `/Game/Blueprints/Car/ArcadeCarController` (`Pawn.GetController` _array_element)))
      (set `/Game/Blueprints/Car/ArcadeCarController.ReverseControls` false _asarcade_car_controller)))
  (`self.K2_DestroyActor`))

(event `self.ReceiveTick`
  (params (DeltaSeconds :type "Float (single-precision)")))

(fn `AddBoost`
  (bind _asarcade_car (cast `/Game/Blueprints/Car/ArcadeCar` (`self.GetOwner`)))
  (if (`/Game/Blueprints/Car/ArcadeCar.IsTouchingGround` _asarcade_car)
    (bind _body (`/Game/Blueprints/Car/ArcadeCar.Body` _asarcade_car))
    (`PrimitiveComponent.SetLinearDamping` _body 3.0)
    (`PrimitiveComponent.AddForce` _body (* (* (`SceneComponent.GetForwardVector` _body) (`/Game/Blueprints/Car/ArcadeCar.forwardForce` _asarcade_car)) 1.5) "None" false)
    (set `self.boostTime` (+ (`self.boostTime`) (`self.boostSubstep`)))
    (else
      (`PrimitiveComponent.SetLinearDamping` _body 0.0))))

(fn `UserConstructionScript`
  (`parent.UserConstructionScript`))