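; Spike trap item that temporarily disables player input on an arcade car that drives over it.
; On BeginPlay it snaps its root to world height zero; a valid overlap blocks the car controller's input, deactivates the hitbox and starts retraction.
; Timers restore input and later re-arm the spike.
; Tick uses Retract and Extend flags to interpolate the cone mesh between sunken and raised absolute world heights.
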(event `self.ReceiveBeginPlay`
  (bind _defaultsceneroot (`self.DefaultSceneRoot`))
  (`parent.ReceiveBeginPlay`)
  (`SceneComponent.K2_SetWorldLocation` _defaultsceneroot (`KismetMathLibrary.MakeVector` (.x (`SceneComponent.K2_GetComponentLocation` _defaultsceneroot)) (.y (`SceneComponent.K2_GetComponentLocation` _defaultsceneroot))) false false))

(event `self.ReceiveActorBeginOverlap`
  (params (OtherActor :type "Actor Object Reference"))
  (if (`self.IsHitboxActive`)
    (bind _asarcade_car (cast `/Game/Blueprints/Car/ArcadeCar` OtherActor))
    (bind _asarcade_car_controller (cast `/Game/Blueprints/Car/ArcadeCarController` (`Pawn.GetController` _asarcade_car)))
    (set `/Game/Blueprints/Car/ArcadeCarController.DisablePlayerInput` true _asarcade_car_controller)
    (`KismetSystemLibrary.K2_SetTimerDelegate` (delegate `EnablePlayerInput`) 3.0)
    (set `self.IsHitboxActive` false)
    (set `self.Retract` true)
    (`KismetSystemLibrary.K2_SetTimerDelegate` (delegate `Reinit`) 5.0)))

(event `EnablePlayerInput`
  (set `/Game/Blueprints/Car/ArcadeCarController.DisablePlayerInput` false (stale `self.ReceiveActorBeginOverlap` _asarcade_car_controller)))

(event `Reinit`
  (set `self.IsHitboxActive` true)
  (set `self.Extend` true))

(event `self.ReceiveTick`
  (params (DeltaSeconds :type "Float (single-precision)"))
  (bind _returnvalue (`SceneComponent.K2_GetComponentLocation` (`self.Cone5`)))
  (bind _returnvalue_2 (`SceneComponent.K2_GetComponentLocation` (`self.Cone5`)))
  (bind _returnvalue_3 (`KismetMathLibrary.VInterpTo` _returnvalue (`KismetMathLibrary.MakeVector` (.x _returnvalue) (.y _returnvalue)) DeltaSeconds 2.0))
  (bind _returnvalue_4 (`KismetMathLibrary.VInterpTo` _returnvalue_2 (`KismetMathLibrary.MakeVector` (.x _returnvalue_2) (.y _returnvalue_2) -101.0) DeltaSeconds 2.0))
  (`parent.ReceiveTick` DeltaSeconds)
  (if (`self.Retract`)
    (`SceneComponent.K2_SetWorldLocation` (`self.Cone5`) _returnvalue_4 true false)
    (if (<= (.z _returnvalue_4) -101.0)
      (set `self.Retract` false))
    (elif (`self.Extend`)
      (`SceneComponent.K2_SetWorldLocation` (`self.Cone5`) _returnvalue_3 true false)
      (if (>= (.z _returnvalue_3) 0.0)
        (set `self.Extend` false)))))

(fn `UserConstructionScript`
  (`parent.UserConstructionScript`))