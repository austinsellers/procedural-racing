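; Throwable item projectile that homes in on an ArcadeCar and launches it into the air.
; It sets its projectile speed on spawn and self-destructs on a timer if nothing is hit.
; The first overlapped car other than its owner becomes the locked homing target.
; Tick checks distance to that target and, when close, replaces the car body's velocity with an upward one and destroys the projectile.
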(event `self.ReceiveBeginPlay`
  (`parent.ReceiveBeginPlay`)
  (set `ProjectileMovementComponent.InitialSpeed` (`self.projectileSpeed`) (`self.ProjectileMovement`))
  (set `ProjectileMovementComponent.MaxSpeed` (`self.projectileSpeed`) (`self.ProjectileMovement`))
  (set `self.canSearchForTarget` true)
  (`KismetSystemLibrary.K2_SetTimerDelegate` (delegate `KillSelf`) 8.0))

(event `KillSelf`
  (`self.K2_DestroyActor`))

(event `self.ReceiveActorBeginOverlap`
  (params (OtherActor :type "Actor Object Reference"))
  (bind _projectilemovement (`self.ProjectileMovement`))
  (`parent.ReceiveActorBeginOverlap` OtherActor)
  (if (`self.canSearchForTarget`)
    (bind _asarcade_car (cast `/Game/Blueprints/Car/ArcadeCar` OtherActor))
    (if (!= _asarcade_car (`self.GetOwner`))
      (set `ProjectileMovementComponent.HomingTargetComponent` (`Actor.RootComponent` _asarcade_car) _projectilemovement)
      (set `ProjectileMovementComponent.bIsHomingProjectile` true _projectilemovement)
      (set `self.canSearchForTarget` false))))

(event `self.ReceiveTick`
  (params (DeltaSeconds :type "Float (single-precision)"))
  (bind _projectilemovement (`self.ProjectileMovement`))
  (bind _returnvalue (`ActorComponent.GetOwner` (`ProjectileMovementComponent.HomingTargetComponent` _projectilemovement)))
  (`parent.ReceiveTick` DeltaSeconds)
  (if (`ProjectileMovementComponent.bIsHomingProjectile` _projectilemovement)
    (if (<= (`self.GetDistanceTo` _returnvalue) 200.0)
      (bind _asarcade_car (cast `/Game/Blueprints/Car/ArcadeCar` _returnvalue))
      (`PrimitiveComponent.SetPhysicsLinearVelocity` (`/Game/Blueprints/Car/ArcadeCar.Body` _asarcade_car) (0.0 0.0 1250.0) false "None")
      (`self.KillSelf`))))

(fn `UserConstructionScript`
  (`parent.UserConstructionScript`))