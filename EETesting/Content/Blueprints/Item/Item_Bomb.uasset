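; Bomb item that is lobbed from its owner and knocks nearby arcade cars away when it goes off.
; On BeginPlay, a force launches its Sphere along the owner's forward and up vectors, and a one-shot timer starts the fuse.
; When the timer fires, it destroys itself, then loops over every ArcadeCar and applies a mass-independent radial push to bodies within range, without distance falloff.
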(event `self.ReceiveBeginPlay`
  (bind _returnvalue (`self.GetOwner`))
  (`parent.ReceiveBeginPlay`)
  (`PrimitiveComponent.AddForce` (`self.Sphere`) (* (+ (`self.GetActorForwardVector` _returnvalue) (`self.GetActorUpVector` _returnvalue)) 20000.0) "None" true)
  (`KismetSystemLibrary.K2_SetTimerDelegate` (delegate `KillSelf`) 4.0))

(event `KillSelf`
  (`self.K2_DestroyActor`)
  (bind _outactors (`GameplayStatics.GetAllActorsOfClass` "/Game/Blueprints/Car/ArcadeCar.ArcadeCar_C"))
  (for _array_element _outactors
    (bind _returnvalue (- (`self.K2_GetActorLocation` _array_element) (`SceneComponent.K2_GetComponentLocation` (`self.Sphere`))))
    (if (< (`KismetMathLibrary.VSize` _returnvalue) 1000.0)
      (`PrimitiveComponent.AddForce` (`/Game/Blueprints/Car/ArcadeCar.Body` _array_element) (* (`KismetMathLibrary.Normal` _returnvalue) 125000.0) "None" true))))

(fn `UserConstructionScript`
  (`parent.UserConstructionScript`))