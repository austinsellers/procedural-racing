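; MasterGameObject sets up local four-player split screen for the arcade car game on BeginPlay.
; InitializeSplitScreen repositions player one's ArcadeCar, then creates each extra local player with an auto-spawned pawn.
; Cars are teleported to staggered offsets along X and raised by SpawnHeight.
; Extra cars get a body material from MaterialArray, and every car is stored in PlayerList.
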(event `self.ReceiveBeginPlay`
  (`self.InitializeSplitScreen` 4 (`self.materialArray`)))

(event `self.ReceiveTick`
  (params (DeltaSeconds :type "Float (single-precision)")))

(fn `InitializeSplitScreen`
  (params (NumberOfPlayers :type Integer) (CharacterMaterialArray :type "Array of Material Object Reference"))
  (bind _asarcade_car (cast `/Game/Blueprints/Car/ArcadeCar` (`GameplayStatics.GetPlayerPawn` 0)))
  (`KismetArrayLibrary.Array_Add` (`self.playerList`) _asarcade_car)
  (bind _rootcomponent (`Actor.RootComponent` _asarcade_car))
  (`SceneComponent.K2_SetWorldLocation` _rootcomponent (+ (`SceneComponent.K2_GetComponentLocation` _rootcomponent) (`KismetMathLibrary.MakeVector` -100.0 0.0 (`self.SpawnHeight`))) false true)
  (for _index (range 1 NumberOfPlayers)
    (bind _returnvalue (`GameplayStatics.CreatePlayer` -1))
    (bind _rootcomponent_2 (`Actor.RootComponent` (`GameplayStatics.GetPlayerPawn` _index)))
    ;[1 1 1] Set Location Other Players
    (`SceneComponent.K2_SetWorldLocation` _rootcomponent_2 (+ (`SceneComponent.K2_GetComponentLocation` _rootcomponent_2) (* (-100.0 0.0 0.0) (+ _index 1)) (`KismetMathLibrary.MakeVector` 0.0 0.0 (`self.SpawnHeight`))) false true)
    (bind _asarcade_car_controller (cast `/Game/Blueprints/Car/ArcadeCarController` _returnvalue))
    (bind _asarcade_car_2 (cast `/Game/Blueprints/Car/ArcadeCar` (`Controller.K2_GetPawn` _asarcade_car_controller)))
    ;[1 1 1] Material Setting
    (`PrimitiveComponent.SetMaterial` (`/Game/Blueprints/Car/ArcadeCar.Body` _asarcade_car_2) 0 (`|GetArrayItem` CharacterMaterialArray (- _index 1)))
    (`KismetArrayLibrary.Array_Add` (`self.playerList`) _asarcade_car_2)))

(fn `UserConstructionScript`)