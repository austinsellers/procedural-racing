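; ArcadeCar is a physics-driven arcade hover car that floats on four hover components initialized at BeginPlay with shared height and strength.
; Throttle applies forward force and damping only when a downward trace finds ground; steering torque scales with forward velocity.
; Each tick a downward trace slows the car over actors tagged "slowdown", and hits on anything but TestRoad add a particle system.
; Two single-use item slots spawn their actor ahead of the car, then empty.
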(event `self.ReceiveBeginPlay`
  (bind _body (`self.Body`))
  (bind _vehicleheight (`self.vehicleHeight`))
  (bind _hoverstrength (`self.hoverStrength`))
  ;[1 1 1] Init Hover Components
  (`/Game/Blueprints/Car/HoverComponent.InitializeHoverComponent` (`self.HoverComponent1`) _body _vehicleheight _hoverstrength)
  (`/Game/Blueprints/Car/HoverComponent.InitializeHoverComponent` (`self.HoverComponent2`) _body _vehicleheight _hoverstrength)
  (`/Game/Blueprints/Car/HoverComponent.InitializeHoverComponent` (`self.HoverComponent3`) _body _vehicleheight _hoverstrength)
  (`/Game/Blueprints/Car/HoverComponent.InitializeHoverComponent` (`self.HoverComponent4`) _body _vehicleheight _hoverstrength))

(event `self.ReceiveTick`
  (params (DeltaSeconds :type "Float (single-precision)"))
  (`self.GetBelowCar`))

(event `self.ReceiveHit`
  (params (MyComp :type "PrimitiveComponent Object Reference") (Other :type "Actor Object Reference") (OtherComp :type "PrimitiveComponent Object Reference") (bSelfMoved :type Boolean) (HitLocation :type "Vector Structure") (HitNormal :type "Vector Structure") (NormalImpulse :type "Vector Structure") (Hit :type "HitResult Structure (by ref)"))
  (cast `/Game/Blueprints/Track/TestRoad` Other
    (:`CastFailed`
      (`AddComponent|NODE_AddParticleSystemComponent-1`))))

(fn `AddForwardForce`
  (params (AxisValue :type "Float (double-precision)"))
  (bind _returnvalue (`SceneComponent.K2_GetComponentLocation` (`self.Body`)))
  ;[1 1 1] Throttle if on ground
  (bind (_outhit _returnvalue_2) (`KismetSystemLibrary.LineTraceSingle` _returnvalue (+ _returnvalue (* (`SceneComponent.GetUpVector` (`self.Body`)) (* (`self.vehicleHeight`) -1.0))) "TraceTypeQuery1"))
  (bind _output_get (set `self.IsTouchingGround` _returnvalue_2))
  (if (and _output_get (`self.CanMove`))
    (`PrimitiveComponent.SetLinearDamping` (`self.Body`) 3.0)
    (`PrimitiveComponent.AddForce` (`self.Body`) (* (* (`SceneComponent.GetForwardVector` (`self.Body`)) (`self.forwardForce`)) AxisValue) "None" false)
    (else
      (`PrimitiveComponent.SetLinearDamping` (`self.Body`) 0.0))))

(fn `AddRightForce`
  (params (RightInput :type "Float (double-precision)"))
  (bind _body (`self.Body`))
  ;[1 1 1] Turn based on linear force
  (bind _returnvalue (`PrimitiveComponent.GetPhysicsLinearVelocity` _body "None"))
  (`PrimitiveComponent.AddTorqueInDegrees` (`self.Body`) (* (`SceneComponent.GetUpVector` (`self.Body`)) (* (`KismetMathLibrary.Dot_VectorVector` _returnvalue (`SceneComponent.GetForwardVector` _body)) RightInput (`self.turningForce`))) "None" false))

(fn `GetBelowCar`
  (bind _returnvalue (`SceneComponent.K2_GetComponentLocation` (`self.Body`)))
  (bind _outhit (`KismetSystemLibrary.LineTraceSingle` _returnvalue (+ _returnvalue (* (`SceneComponent.GetUpVector` (`self.Body`)) (* (`self.vehicleHeight`) -2.0))) "TraceTypeQuery1"))
  (bind (_bblockinghit _binitialoverlap _time _distance _location _impactpoint _normal _impactnormal _physmat _hitactor) (`GameplayStatics.BreakHitResult` _outhit))
  (if (and (`self.ActorHasTag` _hitactor "slowdown") (`KismetSystemLibrary.IsValid` _hitactor))
    (set `self.forwardForce` (* (`self.slowModifier`) (`self.normalSpeed`)))
    (else
      (set `self.forwardForce` (`self.normalSpeed`)))))

(fn `UseItem1`
  (bind _body (`self.Body`))
  ;[1 1 1] Spawn Item in World
  (`|SpawnActorFromClass` (`self.Item1`) (`KismetMathLibrary.MakeTransform` (+ (`SceneComponent.K2_GetComponentLocation` _body) (* (`SceneComponent.GetForwardVector` _body) 100.0)) (`KismetMathLibrary.MakeRotator` 0.0 0.0 (.yaw (`SceneComponent.K2_GetComponentRotation` _body)))) "Undefined" "OverrideRootScale" self self)
  (set `self.Item1` "/Game/Blueprints/Item/Item_None.Item_None_C"))

(fn `UseItem2`
  (bind _body (`self.Body`))
  ;[1 1 1] Spawn Item in World
  (`|SpawnActorFromClass` (`self.Item2`) (`KismetMathLibrary.MakeTransform` (+ (`SceneComponent.K2_GetComponentLocation` _body) (* (`SceneComponent.GetForwardVector` _body) 100.0)) (`KismetMathLibrary.MakeRotator` 0.0 0.0 (.yaw (`SceneComponent.K2_GetComponentRotation` _body)))) "Undefined" "OverrideRootScale" self self)
  (set `self.Item2` "/Game/Blueprints/Item/Item_None.Item_None_C"))

(fn `UserConstructionScript`)