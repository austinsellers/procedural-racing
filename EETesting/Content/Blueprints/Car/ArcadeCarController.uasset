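; Player controller for the arcade car in local 2-4 player play, handling per-player HUD and input.
; On begin play it adds an item HUD, plus main and map HUDs chosen by MasterGameObject's player count.
; It forwards driving (with disable/reverse flags), item use and hold-to-look-back camera to the ArcadeCar.
; A Konami-code check grants speed and items in DevMode, though AddKey, meant to record presses, is empty.
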(event `self.ReceiveBeginPlay`
  (`|ExecutionSequence`
    (:`then_0`
      ;[1 1 1] Add Item HUD to Screen
      (`KismetSystemLibrary.Delay` 0.1)
      (bind _returnvalue (`|CreateWidget` "/Game/Blueprints/UI/HUD_Item.HUD_Item_C" self))
      (bind _output_get (set `self.hud_item` _returnvalue))
      (`UserWidget.AddToPlayerScreen` _output_get 0))
    (:`then_1`
      (bind _outactors (`GameplayStatics.GetAllActorsOfClass` "/Game/Blueprints/MasterGameObject.MasterGameObject_C"))
      (bind _numberofplayers (`/Game/Blueprints/MasterGameObject.numberOfPlayers` (`|GetArrayItem` _outactors)))
      ;[1 1 1] HUD 4P
      (if (== _numberofplayers 4)
        (`KismetSystemLibrary.Delay` 0.1)
        (bind _returnvalue_2 (`|CreateWidget` "/Game/Blueprints/UI/HUD_4P.HUD_4P_C" self))
        (bind _output_get_2 (set `self.HUD_4P` _returnvalue_2))
        (`UserWidget.AddToViewport` _output_get_2 0)
        ;[1 1 1] Add Map HUD
        (`KismetSystemLibrary.Delay` 0.1)
        (bind _returnvalue_3 (`|CreateWidget` "/Game/Blueprints/UI/HUD_MAP_4P.HUD_MAP_4P_C" self))
        (bind _output_get_3 (set `self.HUD_MAP_4P` _returnvalue_3))
        (`UserWidget.AddToViewport` _output_get_3 0)
        (elif (== _numberofplayers 3)
          ;[1 1 1] HUD 3P
          (`KismetSystemLibrary.Delay` 0.1)
          (bind _returnvalue_4 (`|CreateWidget` "/Game/Blueprints/UI/HUD_3P.HUD_3P_C" self))
          (bind _output_get_4 (set `self.HUD_3P` _returnvalue_4))
          (`UserWidget.AddToViewport` _output_get_4 0)
          (`KismetSystemLibrary.Delay` 0.1)
          (bind _returnvalue_5 (`|CreateWidget` "/Game/Blueprints/UI/HUD_MAP_3P.HUD_MAP_3P_C" self))
          (bind _output_get_5 (set `self.HUD_MAP_3P` _returnvalue_5))
          (`UserWidget.AddToViewport` _output_get_5 0)
          (elif (== _numberofplayers 2)
            ;[1 1 1] HUD 2P
            (`KismetSystemLibrary.Delay` 0.1)
            (bind _returnvalue_6 (`|CreateWidget` "/Game/Blueprints/UI/HUD_2P.HUD_2P_C" self))
            (bind _output_get_6 (set `self.HUD_2P` _returnvalue_6))
            (`UserWidget.AddToViewport` _output_get_6 0)
            (`KismetSystemLibrary.Delay` 0.1)
            (bind _returnvalue_7 (`|CreateWidget` "/Game/Blueprints/UI/HUD_MAP_2P.HUD_MAP_2P_C" self))
            (bind _output_get_7 (set `self.HUD_MAP_2P` _returnvalue_7))
            (`UserWidget.AddToViewport` _output_get_7 0)))))))

(event `InputAxis|MoveForward`
  (params (AxisValue :type "Float (single-precision)"))
  ;[1 1 1] Move Car Forward and Back
  (if (not (`self.DisablePlayerInput`))
    (bind _asarcade_car (cast `/Game/Blueprints/Car/ArcadeCar` (`self.K2_GetPawn`)))
    (if (`self.ReverseControls`)
      (bind _result (`/Engine/EditorBlueprintResources/StandardMacros.NegateFloat` AxisValue)
        (:`  `
          (`/Game/Blueprints/Car/ArcadeCar.AddForwardForce` _asarcade_car _result)))
      (else
        (`/Game/Blueprints/Car/ArcadeCar.AddForwardForce` _asarcade_car AxisValue)))))

(event `InputAxis|MoveRight`
  (params (AxisValue :type "Float (single-precision)"))
  ;[1 1 1] Turn Car
  (if (not (`self.DisablePlayerInput`))
    (bind _asarcade_car (cast `/Game/Blueprints/Car/ArcadeCar` (`self.K2_GetPawn`)))
    (if (`self.ReverseControls`)
      (bind _result (`/Engine/EditorBlueprintResources/StandardMacros.NegateFloat` AxisValue)
        (:`  `
          (`/Game/Blueprints/Car/ArcadeCar.AddRightForce` _asarcade_car _result)))
      (else
        (`/Game/Blueprints/Car/ArcadeCar.AddRightForce` _asarcade_car AxisValue)))))

(event `InputAction|UseItem1`
  (params (Key :type "Key Structure"))
  ;[1 1 1] Use Item 1
  (:`Released`
    (bind _asarcade_car (cast `/Game/Blueprints/Car/ArcadeCar` (`self.K2_GetPawn`)))
    (`/Game/Blueprints/Car/ArcadeCar.UseItem1` _asarcade_car)))

(event `InputAction|UseItem2`
  (params (Key :type "Key Structure"))
  ;[1 1 1] Use Item 2
  (:`Released`
    (bind _asarcade_car (cast `/Game/Blueprints/Car/ArcadeCar` (`self.K2_GetPawn`)))
    (`/Game/Blueprints/Car/ArcadeCar.UseItem2` _asarcade_car)))

(event `InputAction|SwitchCamera`
  (params (Key :type "Key Structure"))
  ;[1 1 1] Switch Camera View
  (:`Pressed`
    (set `self.Camera Rotation` (struct :`Pitch` -10.0 :`Yaw` 180.0))
    (set `self.Arm Length` 400.0)
    (bind _asarcade_car (cast `/Game/Blueprints/Car/ArcadeCar` (`self.K2_GetPawn`) :!label _label))
    (bind _springarm (`/Game/Blueprints/Car/ArcadeCar.SpringArm` _asarcade_car))
    (`SceneComponent.K2_SetRelativeRotation` _springarm (`self.Camera Rotation`) false true)
    (set `SpringArmComponent.TargetArmLength` (`self.Arm Length`) _springarm))
  (:`Released`
    (set `self.Camera Rotation` (struct :`Pitch` -10.0))
    (set `self.Arm Length` 600.0)
    (goto _label)))

(event `Key|Up`
  (params (Key :type "Key Structure"))
  ;[1 1 1] Konami Code
  (:`Released`
    (`self.AddKey` "Gamepad_DPad_Up" :!label _label_2)))

(event `Key|Gamepad_DPad_Up`
  (params (Key :type "Key Structure"))
  ;[1 1 1] Konami Code
  (:`Released`
    (goto _label_2)))

(event `Key|Gamepad_FaceButton_Right`
  (params (Key :type "Key Structure"))
  ;[1 1 1] Konami Code
  (:`Released`
    (`self.AddKey` "Gamepad_FaceButton_Right" :!label _label_3)))

(event `Key|B`
  (params (Key :type "Key Structure"))
  ;[1 1 1] Konami Code
  (:`Released`
    (goto _label_3)))

(event `Key|Down`
  (params (Key :type "Key Structure"))
  ;[1 1 1] Konami Code
  (:`Released`
    (`self.AddKey` "Gamepad_DPad_Down" :!label _label_4)))

(event `Key|Gamepad_DPad_Down`
  (params (Key :type "Key Structure"))
  ;[1 1 1] Konami Code
  (:`Released`
    (goto _label_4)))

(event `Key|Gamepad_FaceButton_Bottom`
  (params (Key :type "Key Structure"))
  ;[1 1 1] Konami Code
  (:`Released`
    (`self.AddKey` "Gamepad_FaceButton_Bottom" :!label _label_5)))

(event `Key|V`
  (params (Key :type "Key Structure"))
  ;[1 1 1] Konami Code
  (:`Released`
    (goto _label_5)))

(event `Key|Left`
  (params (Key :type "Key Structure"))
  ;[1 1 1] Konami Code
  (:`Released`
    (`self.AddKey` "Gamepad_DPad_Left" :!label _label_6)))

(event `Key|Gamepad_DPad_Left`
  (params (Key :type "Key Structure"))
  ;[1 1 1] Konami Code
  (:`Released`
    (goto _label_6)))

(event `Key|Gamepad_Special_Right`
  (params (Key :type "Key Structure"))
  (bind _key_combo (`self.Key Combo`))
  ;[1 1 1] Konami Code
  (:`Released`
    (`self.AddKey` "Gamepad_Special_Right" :!label _label_7)
    (for (_array_element _array_index) _key_combo
      (if (`KismetArrayLibrary.Array_IsValidIndex` _key_combo _array_index)
        (if (not (== _array_element (`|GetArrayItem` (`self.Contra Code`) _array_index)))
          (set `self.Correct Input` false)
          (break))
        (else
          (break))))
    (if (`self.Correct Input`)
      (if (`self.DevMode`)
        (bind _asarcade_car (cast `/Game/Blueprints/Car/ArcadeCar` (`self.K2_GetPawn`)))
        (set `/Game/Blueprints/Car/ArcadeCar.normalSpeed` 350000.0 _asarcade_car)
        (set `/Game/Blueprints/Car/ArcadeCar.Item1` "/Game/Blueprints/Item/Item_Spike.Item_Spike_C" _asarcade_car)
        (set `/Game/Blueprints/Car/ArcadeCar.Item2` "/Game/Blueprints/Item/Item_ControlRev.Item_ControlRev_C" _asarcade_car)))
    (`KismetArrayLibrary.Array_Clear` (`self.Key Combo`))
    (set `self.Correct Input` true)))

(event `Key|Enter`
  (params (Key :type "Key Structure"))
  ;[1 1 1] Konami Code
  (:`Released`
    (goto _label_7)))

(event `Key|Gamepad_DPad_Right`
  (params (Key :type "Key Structure"))
  ;[1 1 1] Konami Code
  (:`Released`
    (`self.AddKey` "Gamepad_DPad_Right" :!label _label_8)))

(event `Key|Right`
  (params (Key :type "Key Structure"))
  ;[1 1 1] Konami Code
  (:`Released`
    (goto _label_8)))

(fn `AddKey`
  (params (AddKeyToArray :type "Key Structure")))

(fn `UserConstructionScript`)