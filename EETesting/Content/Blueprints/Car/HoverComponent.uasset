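; Scene component that makes a car hover by acting as a suspension point on a mesh supplied at initialization.
; Each tick it traces down along its up vector and, on a hit, applies a local upward force at its position, fading linearly to zero at trace length.
; It records ground contact in AreWheelsTouching.
; A double-length push-pull variant (AddForceV2) and a forward-drive function remain, but their timer and logic are disconnected.
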(event `InitializeHoverComponent`
  (params (mesh :type "MeshComponent Object Reference") (carHeight :type "Float (double-precision)") (hoverStrength :type "Float (double-precision)"))
  ;[1 1 1] Initilize
  (set `self.MeshComp` mesh)
  (set `self.traceLength` carHeight)
  (set `self.hoverStrength` hoverStrength))

(event `self.ReceiveTick`
  (params (DeltaSeconds :type "Float (single-precision)"))
  (bind _returnvalue (`self.K2_GetComponentLocation`))
  ;[1 1 1] Hover code
  (bind (_outhit _returnvalue_2) (`KismetSystemLibrary.LineTraceSingle` :`Start` _returnvalue :`End` (+ _returnvalue (* (`self.GetUpVector`) (* (`self.traceLength`) -1.0))) :`TraceChannel` "TraceTypeQuery1" :`DrawDebugType` "ForOneFrame"))
  (bind _output_get (set `self.areWheelsTouching` _returnvalue_2))
  (if _output_get
    (`PrimitiveComponent.AddForceAtLocationLocal` (`self.MeshComp`) (* (`KismetMathLibrary.MakeVector` 0.0 0.0 1.0) (`KismetMathLibrary.Lerp` (`self.hoverStrength`) 0.0 (/ (`KismetMathLibrary.VSize` (- (`.Location` (`GameplayStatics.BreakHitResult` _outhit)) (`self.K2_GetComponentLocation`))) (`self.traceLength`)))) (`KismetMathLibrary.TransformLocation` (`self.GetRelativeTransform`)) "None")))

(event `AddForce`
  ;[1 1 1] Hover code
)

(event `AddForceV2`
  (bind _returnvalue (`self.K2_GetComponentLocation`))
  (bind _hoverstrength (`self.hoverStrength`))
  ;[1 1 1] Hover code
  (bind (_outhit _returnvalue_2) (`KismetSystemLibrary.LineTraceSingle` :`Start` _returnvalue :`End` (+ _returnvalue (* (`self.GetUpVector`) (* (`self.traceLength`) -2.0))) :`TraceChannel` "TraceTypeQuery1" :`DrawDebugType` "ForOneFrame"))
  (bind _output_get (set `self.areWheelsTouching` _returnvalue_2))
  (if _output_get
    (`PrimitiveComponent.AddForceAtLocationLocal` (`self.MeshComp`) (* (`KismetMathLibrary.MakeVector` 0.0 0.0 1.0) (`KismetMathLibrary.Lerp` _hoverstrength (* _hoverstrength -1.0) (/ (`KismetMathLibrary.VSize` (- (`.Location` (`GameplayStatics.BreakHitResult` _outhit)) (`self.K2_GetComponentLocation`))) (* (`self.traceLength`) 2.0)))) (`KismetMathLibrary.TransformLocation` (`self.GetRelativeTransform`)) "None")))

(fn `ForwardForce`
  (params (Axis :type "Float (double-precision)"))
  ;[1 1 1] DeadCode
)