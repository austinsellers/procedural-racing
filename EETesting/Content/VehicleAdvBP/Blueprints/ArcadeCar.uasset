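; ArcadeCar is a physics-driven hover vehicle that can carry and use a single item.
; BeginPlay creates the HUD and initializes four hover components on the Body mesh with shared height and strength.
; Throttle adds forward force and damping only when a downward trace finds ground, while steering torque scales with forward velocity.
; UseItem1 spawns the held item class ahead of the car, then clears the slot.
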(event `self.ReceiveBeginPlay`
  (bind _body (`self.Body`))
  (bind _vehicleheight (`self.vehicleHeight`))
  (bind _hoverstrength (`self.hoverStrength`))
  (bind _returnvalue (`|CreateWidget` "/Game/VehicleAdvBP/Blueprints/HUD.HUD_C"))
  (bind _output_get (set `self.hud ref` _returnvalue))
  (`UserWidget.AddToPlayerScreen` _output_get 0)
  (`/Game/VehicleAdvBP/Blueprints/HoverComponent.InitializeHoverComponent` (`self.HoverComponent1`) _body _vehicleheight _hoverstrength)
  (`/Game/VehicleAdvBP/Blueprints/HoverComponent.InitializeHoverComponent` (`self.HoverComponent2`) _body _vehicleheight _hoverstrength)
  (`/Game/VehicleAdvBP/Blueprints/HoverComponent.InitializeHoverComponent` (`self.HoverComponent3`) _body _vehicleheight _hoverstrength)
  (`/Game/VehicleAdvBP/Blueprints/HoverComponent.InitializeHoverComponent` (`self.HoverComponent4`) _body _vehicleheight _hoverstrength))

(event `self.ReceiveTick`
  (params (DeltaSeconds :type "Float (single-precision)"))
  (`KismetSystemLibrary.PrintString` (`KismetSystemLibrary.GetClassDisplayName` (`self.Item1`)) true true (struct :`G` 0.66 :`B` 1.0 :`A` 1.0) DeltaSeconds))

(fn `AddForwardForce`
  (params (AxisValue :type "Float (double-precision)"))
  (bind _returnvalue (`SceneComponent.K2_GetComponentLocation` (`self.Body`)))
  ;[1 1 1] Throttle if on ground
  (bind (_outhit _returnvalue_2) (`KismetSystemLibrary.LineTraceSingle` :`Start` _returnvalue :`End` (+ _returnvalue (* (`SceneComponent.GetUpVector` (`self.Body`)) (* (`self.vehicleHeight`) -2.0))) :`TraceChannel` "TraceTypeQuery1" :`DrawDebugType` "ForOneFrame"))
  (bind _output_get (set `self.IsTouchingGround` _returnvalue_2))
  (if (and _output_get (`self.CanMove`))
    (`PrimitiveComponent.SetLinearDamping` (`self.Body`) 3.0)
    (`PrimitiveComponent.AddForce` (`self.Body`) (* (* (`SceneComponent.GetForwardVector` (`self.Body`)) (`self.forwardForce`)) AxisValue) "None" false)
    (else
      (`PrimitiveComponent.SetLinearDamping` (`self.Body`) 0.0))))

(fn `AddRightForce`
  (params (RightInput :type "Float (double-precision)"))
  (bind _body (`self.Body`))
  ;[1 1 1] Turn based on linear force
  (bind _returnvalue (`PrimitiveComponent.GetPhysicsLinearVelocity` _body "None"))
  (`PrimitiveComponent.AddTorqueInDegrees` (`self.Body`) (* (`SceneComponent.GetUpVector` (`self.Body`)) (* (`KismetMathLibrary.Dot_VectorVector` _returnvalue (`SceneComponent.GetForwardVector` _body)) RightInput (`self.turningForce`))) "None" false))

(fn `UseItem1`
  (bind _body (`self.Body`))
  (`|SpawnActorFromClass` (`self.Item1`) (`KismetMathLibrary.MakeTransform` (+ (`SceneComponent.K2_GetComponentLocation` _body) (* (`SceneComponent.GetForwardVector` _body) 100.0)) (`KismetMathLibrary.MakeRotator` 0.0 0.0 (.yaw (`SceneComponent.K2_GetComponentRotation` _body)))) "Undefined" "OverrideRootScale" self self)
  (set `self.Item1` "/Game/Items/Item_None.Item_None_C"))

(fn `UserConstructionScript`)