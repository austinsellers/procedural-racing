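; TestRoad is a road segment actor that grows a trail behind ArcadeCars and scores the driver.
; When a car first stops overlapping it, it spawns the next TestRoad just ahead at zero height, matching the car's yaw and body material, and increments that player's MasterGameObject score.
; Each segment increments a track number, triggering a delayed row of three RandomItemPickups every hundredth segment.
; Logic for destroying other players' overlapping segments is unconnected.
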(event `self.ReceiveActorEndOverlap`
  (params (OtherActor :type "Actor Object Reference"))
  ;[1 1 1] Testing Road Generation
  (bind _asarcade_car (cast `/Game/VehicleAdvBP/Blueprints/ArcadeCar` OtherActor))
  (if (`self.firstPlace`)
    (set `self.playerRef` _asarcade_car)
    (set `self.firstPlace` false)
    (bind _body (`/Game/VehicleAdvBP/Blueprints/ArcadeCar.Body` _asarcade_car))
    (bind _returnvalue (`|SpawnActorFromClass` "TestRoad_C" (`KismetMathLibrary.MakeTransform` (+ (* (`KismetMathLibrary.Normal` (`KismetMathLibrary.MakeVector` (.x (`SceneComponent.GetForwardVector` _body)) (.y (`SceneComponent.GetForwardVector` _body)))) 50.0) (`KismetMathLibrary.MakeVector` (.x (`SceneComponent.K2_GetComponentLocation` _body)) (.y (`SceneComponent.K2_GetComponentLocation` _body)))) (`KismetMathLibrary.MakeRotator` 0.0 0.0 (.yaw (`SceneComponent.K2_GetComponentRotation` (`/Game/VehicleAdvBP/Blueprints/ArcadeCar.Body` _asarcade_car)))) (.scale (`SceneComponent.K2_GetComponentToWorld` (`self.Arrow`)))) "AlwaysSpawn" "OverrideRootScale" null null))
    (`PrimitiveComponent.SetMaterial` (`StaticMeshActor.StaticMeshComponent` _returnvalue) 0 (`PrimitiveComponent.GetMaterial` (`/Game/VehicleAdvBP/Blueprints/ArcadeCar.Body` _asarcade_car) 0))
    (bind _output_get (set `/Game/VehicleAdvBP/Blueprints/TestRoad.trackNumber` (+ (`self.trackNumber`) 1) _returnvalue))
    (if (== (mod _output_get 100) 0)
      (`KismetSystemLibrary.K2_SetTimer` null "SpawnPickups" 1.0))
    ;[1 1 1] Add Score
    (bind _outactors (`GameplayStatics.GetAllActorsOfClass` "/Game/VehicleAdvBP/Blueprints/MasterGameObject.MasterGameObject_C"))
    (bind _asmaster_game_object (cast `/Game/VehicleAdvBP/Blueprints/MasterGameObject` (`|GetArrayItem` _outactors)))
    (bind _playerscore (`/Game/VehicleAdvBP/Blueprints/MasterGameObject.playerScore` _asmaster_game_object))
    (bind _returnvalue_2 (`KismetArrayLibrary.Array_Find` (`/Game/VehicleAdvBP/Blueprints/MasterGameObject.playerList` _asmaster_game_object) (`self.playerRef`)))
    (`KismetArrayLibrary.Array_Set` _playerscore _returnvalue_2 (+ (`|GetArrayItem` _playerscore _returnvalue_2) 1))))

(event `self.ReceiveBeginPlay`)

(event `self.ReceiveActorBeginOverlap`
  (params (OtherActor :type "Actor Object Reference")))

(event `self.ReceiveTick`
  (params (DeltaSeconds :type "Float (single-precision)")))

(fn `SpawnPickups`
  (`|SpawnActorFromClass` "/Game/Items/RandomItemPickup.RandomItemPickup_C" (`KismetMathLibrary.MakeTransform` (`KismetMathLibrary.MakeVector` (.x (+ (.location (`self.GetTransform`)) (* (`SceneComponent.GetRightVector` (`self.StaticMeshComponent`)) 300.0))) (.y (+ (.location (`self.GetTransform`)) (* (`SceneComponent.GetRightVector` (`self.StaticMeshComponent`)) 300.0))) (+ (.z (+ (.location (`self.GetTransform`)) (* (`SceneComponent.GetRightVector` (`self.StaticMeshComponent`)) 300.0))) 100.0)) (.rotation (`self.GetTransform`)) (.scale (`self.GetTransform`))) "Undefined" "OverrideRootScale" null null)
  (`|SpawnActorFromClass` "/Game/Items/RandomItemPickup.RandomItemPickup_C" (`KismetMathLibrary.MakeTransform` (`KismetMathLibrary.MakeVector` (.x (+ (.location (`self.GetTransform`)) (* (`SceneComponent.GetRightVector` (`self.StaticMeshComponent`)) -300.0))) (.y (+ (.location (`self.GetTransform`)) (* (`SceneComponent.GetRightVector` (`self.StaticMeshComponent`)) -300.0))) (+ (.z (+ (.location (`self.GetTransform`)) (* (`SceneComponent.GetRightVector` (`self.StaticMeshComponent`)) -300.0))) 100.0)) (.rotation (`self.GetTransform`)) (.scale (`self.GetTransform`))) "Undefined" "OverrideRootScale" null null)
  (`|SpawnActorFromClass` "/Game/Items/RandomItemPickup.RandomItemPickup_C" (`KismetMathLibrary.MakeTransform` (`KismetMathLibrary.MakeVector` (.x (.location (`self.GetTransform`))) (.y (.location (`self.GetTransform`))) (+ (.z (.location (`self.GetTransform`))) 100.0)) (.rotation (`self.GetTransform`)) (.scale (`self.GetTransform`))) "Undefined" "OverrideRootScale" null null))

(fn `UserConstructionScript`)